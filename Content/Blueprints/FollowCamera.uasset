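; FollowCamera is a shared camera actor that keeps two cars in frame, set as view target for player controllers 0 and 1.
; BeginPlay stores the first CarModel1 and CarModel2 actors; an AISedan fallback exists behind a hard-coded true branch.
; Each tick it moves to the midpoint between the cars and scales the camera arm length from their clamped separation.
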(event `self.ReceiveBeginPlay`
  ;[1 1 1] Make both characters use the camera component of FollowCamera
  (`PlayerController.SetViewTargetWithBlend` (`GameplayStatics.GetPlayerController` 1) self 0.0 "VTBlend_Linear" 0.0 false)
  (`PlayerController.SetViewTargetWithBlend` (`GameplayStatics.GetPlayerController` 0) self 0.0 "VTBlend_Linear" 0.0 false)
  ;[1 1 1] Store references to both cars in variables
  (`|ExecutionSequence`
    (:`then_0`
      (bind _outactors (`GameplayStatics.GetAllActorsOfClass` "/Game/Blueprints/VehicleBlueprints/CarModel1.CarModel1_C"))
      (set `self.Car1` (`KismetArrayLibrary.Array_Get` _outactors)))
    (:`then_1`
      (if true
        (bind _outactors_2 (`GameplayStatics.GetAllActorsOfClass` "/Game/Blueprints/VehicleBlueprints/CarModel2.CarModel2_C"))
        (set `self.Car2` (`KismetArrayLibrary.Array_Get` _outactors_2))
        (else
          (bind _outactors_3 (`GameplayStatics.GetAllActorsOfClass` "/Game/Vehicle/AISedan/AI/AISedan.AISedan_C"))
          (set `self.Car2` (`KismetArrayLibrary.Array_Get` _outactors_3)))))))

(event `self.ReceiveActorBeginOverlap`
  (params (OtherActor :type "Actor Object Reference")))

(event `self.ReceiveTick`
  (params (DeltaSeconds :type "Float (single-precision)"))
  (bind _distance (`self.Distance`))
  ;[1 1 1] Gets the location for both cars, and determines the distance between them.
  (set `self.Distance` (- (`self.K2_GetActorLocation` (`self.Car1`)) (`self.K2_GetActorLocation` (`self.Car2`))))
  ;[1 1 1] Adjust the camera, depending on the distance between the two cars.
  (`self.K2_SetActorLocation` (+ (`self.K2_GetActorLocation` (`self.Car2`)) (/ _distance 2)))
  (bind _output_get (set `SpringArmComponent.TargetArmLength` (* (`KismetMathLibrary.FClamp` (`KismetMathLibrary.VSize` _distance) (`self.MinimumCameraDistance`) (`self.MaximumCameraDistance`)) 1.8) (`self.CameraArm`))))

(fn `NewFunction_0`)

(fn `NewFunction_1`)

(fn `UserConstructionScript`)