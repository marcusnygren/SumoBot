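; SumoBotGameMode is the game mode that assigns players to cars and sets up the camera at level start.
; On BeginPlay, player 0 possesses the first CarModel1, then a switch on level name picks the setup.
; Multiplayer levels create a second local player to possess the first CarModel2.
; Both multiplayer and singleplayer levels then spawn a FollowCamera stored as FocusCamera, while unlisted levels only print a debug message.
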(event `self.ReceiveTick`
  (params (DeltaSeconds :type "Float (single-precision)")))

(event `self.ReceiveBeginPlay`
  (`KismetSystemLibrary.PrintString` "MultiPlayerGameMode: Event BeginPlay")
  ;[1 1 1] Create the first controller, which controls player1
  (bind _outactors (`GameplayStatics.GetAllActorsOfClass` "/Game/Blueprints/VehicleBlueprints/CarModel1.CarModel1_C"))
  (`Controller.Possess` (`GameplayStatics.GetPlayerController` 0) (`KismetArrayLibrary.Array_Get` _outactors))
  ;[1 1 1] Check which level is activated
  (bind _returnvalue (`GameplayStatics.GetCurrentLevelName` true))
  (switch `string` _returnvalue ; Checking which level is activated
    (:`Default`
      (`KismetSystemLibrary.PrintString` "Kommer jag hit? för menyn eventuellt???" true true (struct :`G` 0.66 :`B` 1.0 :`A` 1.0) 10.0))
    (:`LevelAMultiplayer`
      ;[1 1 1] If multiplayer, spawn another controller
      (bind _returnvalue_2 (`GameplayStatics.CreatePlayer` -1 :!label _label))
      (bind _outactors_2 (`GameplayStatics.GetAllActorsOfClass` "/Game/Blueprints/VehicleBlueprints/CarModel2.CarModel2_C"))
      (`Controller.Possess` _returnvalue_2 (`KismetArrayLibrary.Array_Get` _outactors_2))
      ;[1 1 1] Spawn the camera
      (bind _returnvalue_3 (`|SpawnActorFromClass` "/Game/Blueprints/FollowCamera.FollowCamera_C" (`self.GetTransform`) "Undefined" "OverrideRootScale" :!label _label_2))
      (set `self.FocusCamera` _returnvalue_3))
    (:`LevelBMultiplayer`
      (goto _label))
    (:`LevelASingleplayer`
      (goto _label_2))
    (:`LevelBSingleplayer`
      (goto _label_2))
    (:`LevelCSingleplayer`
      (goto _label_2))))

(fn `UserConstructionScript`)