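; Single-player game mode that puts the player in a CarModel1 car and creates a follow camera.
; On every Tick, with no one-time guard, it has player 0 possess the first CarModel1 found, calls CreatePlayer and spawns a new FollowCamera stored as FocusCamera.
; BeginPlay is empty, and a branch that would spawn the car at the player start is disconnected.
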(event `/Game/Blueprints/SumoBotMode.ReceiveBeginPlay`)

(event `self.ReceiveTick`
  (params (DeltaSeconds :type "Float (single-precision)"))
  (bind _outactors (`GameplayStatics.GetAllActorsOfClass` "/Game/Blueprints/VehicleBlueprints/CarModel1.CarModel1_C"))
  (`Controller.Possess` (`GameplayStatics.GetPlayerController` 0) (`KismetArrayLibrary.Array_Get` _outactors))
  (`GameplayStatics.CreatePlayer` -1)
  (bind _returnvalue (`|SpawnActorFromClass` "/Game/Blueprints/FollowCamera.FollowCamera_C" (`self.GetTransform`) "Undefined" "OverrideRootScale"))
  (set `self.FocusCamera` _returnvalue))

(fn `UserConstructionScript`)