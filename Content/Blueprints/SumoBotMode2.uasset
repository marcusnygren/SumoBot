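; SumoBotMode2 sets up a local two-player session for what appears to be a sumo-style car game.
; On BeginPlay it has player controller 0 possess the first existing CarModel1, then creates a second local player to possess the first existing CarModel2.
; It then spawns a FollowCamera at its own transform and stores it as FocusCamera.
; Disconnected leftover nodes for player-start car spawning and debug printing never run.
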(event `/Game/Blueprints/SumoBotMode.ReceiveTick`
  (params (DeltaSeconds :type "Float (single-precision)")))

(event `/Game/Blueprints/SumoBotMode.ReceiveBeginPlay`
  (bind _outactors (`GameplayStatics.GetAllActorsOfClass` "/Game/Blueprints/VehicleBlueprints/CarModel1.CarModel1_C"))
  (`Controller.Possess` (`GameplayStatics.GetPlayerController` 0) (`KismetArrayLibrary.Array_Get` _outactors))
  (bind _returnvalue (`GameplayStatics.CreatePlayer` -1))
  (bind _outactors_2 (`GameplayStatics.GetAllActorsOfClass` "/Game/Blueprints/VehicleBlueprints/CarModel2.CarModel2_C"))
  (`Controller.Possess` _returnvalue (`KismetArrayLibrary.Array_Get` _outactors_2))
  (bind _outactors_3 (`GameplayStatics.GetAllActorsOfClass` "/Game/Blueprints/VehicleBlueprints/CarModel1.CarModel1_C"))
  (bind _returnvalue_2 (`|SpawnActorFromClass` "/Game/Blueprints/FollowCamera.FollowCamera_C" (`self.GetTransform`) "Undefined" "OverrideRootScale"))
  (set `self.FocusCamera` _returnvalue_2))

(fn `UserConstructionScript`)