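; SumoBotMode is the game mode for a two-player local sumo bot match, setting up both cars and a camera.
; On BeginPlay it spawns CarModel1 for player controller 0, then creates a second local player to possess a CarModel2, placing each at a found PlayerStart.
; It also prints the CarModel1 count, then spawns a FollowCamera and stores it as FocusCamera.
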(event `self.ReceiveBeginPlay`
  (bind _returnvalue (`|SpawnActorFromClass` "/Game/Blueprints/VehicleBlueprints/CarModel1.CarModel1_C" (`self.GetTransform` (`self.K2_FindPlayerStart` null)) "Undefined" "OverrideRootScale"))
  (`Controller.Possess` (`GameplayStatics.GetPlayerController` 0) _returnvalue)
  (bind _returnvalue_2 (`GameplayStatics.CreatePlayer` -1))
  (bind _returnvalue_3 (`|SpawnActorFromClass` "/Game/Blueprints/VehicleBlueprints/CarModel2.CarModel2_C" (`self.GetTransform` (`self.K2_FindPlayerStart` null)) "Undefined" "OverrideRootScale"))
  (`Controller.Possess` _returnvalue_2 _returnvalue_3)
  (bind _outactors (`GameplayStatics.GetAllActorsOfClass` "/Game/Blueprints/VehicleBlueprints/CarModel1.CarModel1_C"))
  (`KismetSystemLibrary.PrintString` (`KismetStringLibrary.Conv_IntToString` (`KismetArrayLibrary.Array_Length` _outactors)))
  (bind _returnvalue_4 (`|SpawnActorFromClass` "/Game/Blueprints/FollowCamera.FollowCamera_C" (`self.GetTransform`) "Undefined" "OverrideRootScale"))
  (set `self.FocusCamera` _returnvalue_4))

(event `self.ReceiveTick`
  (params (DeltaSeconds :type "Float (single-precision)")))

(fn `UserConstructionScript`)